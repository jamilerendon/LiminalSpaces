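; Boss projectile for Anemoia that damages the third-person player character when it touches them.
; Overlap with component E caches the character, spawns a splash effect at its capsule and passes through a DoOnce gate to apply fixed damage.
; Ending the overlap waits briefly, then fires the beam-attack reset event to reopen the gate, preventing repeated hits in quick succession.
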(event `self.ReceiveBeginPlay`)

(event `reset beam attack fire state`
  (goto _label :!via `Reset`))

(event `self.e.OnComponentBeginOverlap`
  (params (OverlappedComponent :type "PrimitiveComponent Object Reference") (OtherActor :type "Actor Object Reference") (OtherComp :type "PrimitiveComponent Object Reference") (OtherBodyIndex :type Integer) (bFromSweep :type Boolean) (SweepResult :type "HitResult Structure (by ref)"))
  (bind _asbp_third_person_character (cast `/Game/ThirdPerson/Blueprints/BP_ThirdPersonCharacter` OtherActor))
  (bind _output_get (set `self.As BP Third Person Character` _asbp_third_person_character))
  (`NiagaraFunctionLibrary.SpawnSystemAtLocation` "/Game/NiagaraSystems/NS_Splash.NS_Splash" (`SceneComponent.K2_GetComponentLocation` (`Character.CapsuleComponent` _output_get)))
  (`/Engine/EditorBlueprintResources/StandardMacros.DoOnce` false :!label _label
    (:`Completed`
      (`/Game/ThirdPerson/Blueprints/I_Interactions.RecieveDamage` _asbp_third_person_character 35.0 null)
      (`/Game/ThirdPerson/Blueprints/I_Interactions.RecieveDamage` _output_get 35.0 null))))

(event `self.e.OnComponentEndOverlap`
  (params (OverlappedComponent :type "PrimitiveComponent Object Reference") (OtherActor :type "Actor Object Reference") (OtherComp :type "PrimitiveComponent Object Reference") (OtherBodyIndex :type Integer))
  (cast `/Game/ThirdPerson/Blueprints/BP_ThirdPersonCharacter` OtherActor)
  (`KismetSystemLibrary.Delay` 0.6)
  (`self.reset beam attack fire state`))

(fn `UserConstructionScript`)