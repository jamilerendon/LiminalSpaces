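; Anemoia boss enemy that hunts the player with ranged, melee and scream attacks.
; Until it sees the player, Tick moves it toward them and triggers a cooldown-limited knockback scream at close range.
; Pawn sensing starts a DoOnce-gated attack cycle, randomly choosing lunge or projectile when far, and montage combos when near.
; Helper functions toggle socket-attached hitboxes and set damage tiers; the teleport effect sequence is unconnected.
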(event `self.ReceiveBeginPlay`
  (`parent.ReceiveBeginPlay`)
  (set `self.DeathMontage` "/Game/Characters/BossImplementation/RM_Anemoia/SkeletalMeshes/RM_AnemoiaDeath_Montage.RM_AnemoiaDeath_Montage")
  (set `self.Who` self)
  (`SceneComponent.K2_AttachToComponent` (`self.Cube`) (`self.Mesh`) "hand_LSocket" "SnapToTarget" "SnapToTarget" "KeepRelative" true)
  (`PrimitiveComponent.SetCollisionEnabled` (`self.LeftHand`) "NoCollision")
  (`SceneComponent.K2_AttachToComponent` (`self.StaticMesh`) (`self.Mesh`) "hand_RSocket" "SnapToTarget" "SnapToTarget" "KeepRelative" true)
  (`PrimitiveComponent.SetCollisionEnabled` (`self.RightHand`) "NoCollision")
  (`SceneComponent.K2_AttachToComponent` (`self.StaticMesh1`) (`self.Mesh`) "rootSocket" "SnapToTarget" "SnapToTarget" "KeepRelative" true)
  (`PrimitiveComponent.SetCollisionEnabled` (`self.BothHands`) "NoCollision")
  (`SceneComponent.SetHiddenInGame` (`self.StaticMesh1`) true false)
  (`SceneComponent.SetHiddenInGame` (`self.StaticMesh`) true false)
  (`SceneComponent.SetHiddenInGame` (`self.Cube`) true false)
  (`PrimitiveComponent.SetCollisionEnabled` (`self.KnockbackScream`) "NoCollision"))

(event `self.ReceiveTick`
  (params (DeltaSeconds :type "Float (single-precision)"))
  (if (`self.BossIsDead`)
    _
    (elif (not (`self.IsSeeingPlayer`))
      (bind _returnvalue (`GameplayStatics.GetActorOfClass` "/Game/ThirdPerson/Blueprints/BP_ThirdPersonCharacter.BP_ThirdPersonCharacter_C"))
      (set `self.Player` _returnvalue)
      (`self.FocusThePlayerAndDoVFX`)
      (if (not (`self.IsSeeingPlayer`))
        (bind _yes (`self.BossIsClose`))
        (if _yes
          (`/Engine/EditorBlueprintResources/StandardMacros.DoOnce` false :!label _label
            (:`Completed`
              (`self.ScreamAttack`))))))))

(event `ResetScreamPossibility`
  (`KismetSystemLibrary.Delay` 15.0)
  (goto _label :!via `Reset`))

(event `self.PawnSensing.OnSeePawn`
  (params (Pawn :type "Pawn Object Reference"))
  (if (not (`self.BossIsDead`))
    (bind _output_get (set `self.IsSeeingPlayer` true))
    (if _output_get
      (`/Engine/EditorBlueprintResources/StandardMacros.DoOnce` false :!label _label_2
        (:`Completed`
          (`self.FollowPlayer`))))))

(event `Reset Follow Player`
  (set `self.IsSeeingPlayer` false)
  (goto _label_2 :!via `Reset`))

(event `FollowPlayer`
  (if (not (`self.BossIsDead`))
    (bind _output_get (set `self.canAttack` true))
    (if _output_get
      (`self.DeactivateScreamHitbox`)
      (bind _returnvalue (`GameplayStatics.GetActorOfClass` "/Game/ThirdPerson/Blueprints/BP_ThirdPersonCharacter.BP_ThirdPersonCharacter_C"))
      (if (> (`KismetMathLibrary.Vector_Distance` (`SceneComponent.K2_GetComponentLocation` (`self.CapsuleComponent`)) (`SceneComponent.K2_GetComponentLocation` (`Character.Mesh` _returnvalue))) 800.0)
        (`/Engine/EditorBlueprintResources/StandardMacros.DoOnce` false :!label _label_3
          (:`Completed`
            (if (`self.canAttack`)
              (set `self.canAttack` false)
              (if (`KismetMathLibrary.RandomBool`)
                (`self.Setup Lunge`)
                (`self.PlayAnimMontage` "/Game/Characters/BossImplementation/RM_Anemoia/SkeletalMeshes/RM_AnemoiaLunge_Montage.RM_AnemoiaLunge_Montage")
                (`KismetSystemLibrary.Delay` 1.0)
                (`MovementComponent.StopMovementImmediately` (`self.CharacterMovement`))
                (`self.LaunchCharacter` (`KismetMathLibrary.MakeVector` (.x (`self.LungeCapacity`)) (.y (`self.LungeCapacity`)) 100.0) true)
                (`KismetSystemLibrary.Delay` 0.9)
                (`self.Reset Lunge`)
                (`self.Reset Follow Player`)
                (else
                  (`self.Throw Projectile`)
                  (bind _returnvalue_2 (`self.PlayAnimMontage` "/Game/Characters/BossImplementation/RM_Anemoia/SkeletalMeshes/RM_AnemoiaThrow_Montage.RM_AnemoiaThrow_Montage"))
                  (`KismetSystemLibrary.Delay` _returnvalue_2)
                  (`self.Reset Lunge`)
                  (`self.Reset Follow Player`))))))
        (else
          (`KismetSystemLibrary.Delay` 0.4)
          (`|AIMoveTo` self (0.0 0.0 0.0) (`GameplayStatics.GetPlayerCharacter` 0) 350.0
            (:`OnSuccess`
              (`MovementComponent.StopMovementImmediately` (`self.CharacterMovement`))
              (`/Engine/EditorBlueprintResources/StandardMacros.DoOnce` false :!label _label_4
                (:`Completed`
                  (if (`self.canAttack`)
                    (set `self.canAttack` false)
                    (if (`KismetMathLibrary.RandomBool`)
                      (bind _returnvalue_3 (`self.PlayAnimMontage` "/Game/Characters/BossImplementation/RM_Anemoia/SkeletalMeshes/RM_Anemoia1HandSlam_Montage.RM_Anemoia1HandSlam_Montage"))
                      (`KismetSystemLibrary.Delay` _returnvalue_3)
                      (if (`KismetMathLibrary.RandomBool`)
                        (`self.ResetAttack`)
                        (`self.Reset Follow Player`)
                        (else
                          (bind _returnvalue_4 (`self.PlayAnimMontage` "/Game/Characters/BossImplementation/RM_Anemoia/SkeletalMeshes/RM_AnemoiaUppercut_Montage.RM_AnemoiaUppercut_Montage"))
                          (`KismetSystemLibrary.Delay` _returnvalue_4)
                          (`self.ResetAttack`)
                          (`self.Reset Follow Player`)))
                      (else
                        (bind _returnvalue_5 (`self.PlayAnimMontage` "/Game/Characters/BossImplementation/RM_Anemoia/SkeletalMeshes/RM_AnemoiaSlashCombo1_Montage.RM_AnemoiaSlashCombo1_Montage"))
                        (`KismetSystemLibrary.Delay` _returnvalue_5)
                        (bind _returnvalue_6 (`self.PlayAnimMontage` "/Game/Characters/BossImplementation/RM_Anemoia/SkeletalMeshes/RM_AnemoiaSlashCombo2_Montage.RM_AnemoiaSlashCombo2_Montage"))
                        (`self.FocusThePlayerAndDoVFX`)
                        (`KismetSystemLibrary.Delay` _returnvalue_6)
                        (if (`KismetMathLibrary.RandomBool`)
                          (bind _returnvalue_7 (`self.PlayAnimMontage` "/Game/Characters/BossImplementation/RM_Anemoia/SkeletalMeshes/RM_AnemoiaSlashCombo3_Montage.RM_AnemoiaSlashCombo3_Montage"))
                          (`KismetSystemLibrary.Delay` _returnvalue_7)
                          (`self.ResetAttack`)
                          (`self.Reset Follow Player`)
                          (else
                            (bind _returnvalue_8 (`self.PlayAnimMontage` "/Game/Characters/BossImplementation/RM_Anemoia/SkeletalMeshes/RM_AnemoiaUppercut_Montage.RM_AnemoiaUppercut_Montage"))
                            (`KismetSystemLibrary.Delay` _returnvalue_8)
                            (`self.ResetAttack`)
                            (`self.Reset Follow Player`)))))))))))))))

(event `ResetAttack`
  (goto _label_4 :!via `Reset`))

(event `ScreamAttack`
  (`MovementComponent.StopMovementImmediately` (`self.CharacterMovement`))
  (bind _returnvalue (`self.PlayAnimMontage` "/Game/Characters/BossImplementation/RM_Anemoia/SkeletalMeshes/RM_AnemoiaScream_Montage.RM_AnemoiaScream_Montage" 1.5))
  (`KismetSystemLibrary.Delay` (/ _returnvalue 4.0))
  (`self.LaunchCharacter` (`self.Player`) (1400.0 1400.0 100.0) true false)
  (`KismetSystemLibrary.Delay` (/ _returnvalue 2.0))
  (bind _yes (`self.BossIsClose`))
  (if _yes
    (`self.ResetScreamPossibility`)
    (else
      (`self.ResetScreamPossibility`))))

(event `Reset Lunge`
  (goto _label_3 :!via `Reset`))

(event `Throw Projectile`
  (bind _returnvalue (`SceneComponent.GetSocketLocation` (`self.Mesh`) "hand_lSocket"))
  (bind _returnvalue_2 (`GameplayStatics.GetActorOfClass` "/Game/ThirdPerson/Blueprints/BP_ThirdPersonCharacter.BP_ThirdPersonCharacter_C"))
  (`|SpawnActorFromClass` "/Game/Characters/BossImplementation/BP_MasterProjectile.BP_MasterProjectile_C" (`KismetMathLibrary.MakeTransform` _returnvalue (`KismetMathLibrary.MakeRotFromX` (`KismetMathLibrary.Normal` (- (`SceneComponent.K2_GetComponentLocation` (`Character.Mesh` _returnvalue_2)) _returnvalue)))) "Undefined" "MultiplyWithRoot" null null))

(event `Setup Lunge`
  (bind _returnvalue (`GameplayStatics.GetActorOfClass` "/Game/ThirdPerson/Blueprints/BP_ThirdPersonCharacter.BP_ThirdPersonCharacter_C"))
  (set `self.LungeCapacity` (* (`KismetMathLibrary.Normal` (- (`SceneComponent.K2_GetComponentLocation` (`Character.Mesh` _returnvalue)) (`SceneComponent.K2_GetComponentLocation` (`self.CapsuleComponent`)))) 4000.0)))

(event `FoucsPlayer`
  (`AIController.K2_SetFocus` (`AIBlueprintHelperLibrary.GetAIController` self) (`self.Player`)))

(event `FocusThePlayerAndDoVFX`
  (if (not (`self.IsSeeingPlayer`))
    (`self.MoveToPlayerLocation`)))

(event `UnFocusPlayer`
  (`AIController.K2_SetFocus` (`AIBlueprintHelperLibrary.GetAIController` self) null))

(event `MoveToPlayerLocation`
  (`|AIMoveTo` self (`self.K2_GetActorLocation` (`self.Player`)) null 10.0))

(fn `ActivateAttackLeftHitbox`
  (`PrimitiveComponent.SetCollisionEnabled` (`self.LeftHand`) "QueryAndPhysics"))

(fn `ActivateAttackRightHitbox`
  (`PrimitiveComponent.SetCollisionEnabled` (`self.RightHand`) "QueryAndPhysics"))

(fn `ActivateBothHands`
  (`PrimitiveComponent.SetCollisionEnabled` (`self.BothHands`) "QueryAndPhysics"))

(fn `ActivateScreamHitbox`
  (`PrimitiveComponent.SetCollisionEnabled` (`self.KnockbackScream`) "QueryAndPhysics")
  (`NiagaraFunctionLibrary.SpawnSystemAttached` "/Game/NiagaraSystems/Shockwave/NS_Shockwave.NS_Shockwave" (`self.Mesh`) "headSocket" (0.0 0.0 0.0) (struct) "KeepRelativeOffset" true))

(fn `ChangeMaterialBack`
  (`PrimitiveComponent.SetMaterial` (`self.Mesh`) 0 "/Game/Characters/BossImplementation/RM_Anemoia/Materials/AnemoiaMat.AnemoiaMat"))

(fn `DeactivateAttackLeftHitbox`
  (`PrimitiveComponent.SetCollisionEnabled` (`self.LeftHand`) "NoCollision"))

(fn `DeactivateAttackRightHitbox`
  (`PrimitiveComponent.SetCollisionEnabled` (`self.RightHand`) "NoCollision"))

(fn `DeactivateBothHands`
  (`PrimitiveComponent.SetCollisionEnabled` (`self.BothHands`) "NoCollision"))

(fn `DeactivateScreamHitbox`
  (`PrimitiveComponent.SetCollisionEnabled` (`self.KnockbackScream`) "NoCollision"))

(fn `FixRotation`
  (params (Player :type "Pawn Object Reference"))
  (`/Engine/EditorBlueprintResources/StandardMacros.DoOnce` false
    (:`Completed`
      (`self.K2_SetActorRotation` (`self.K2_GetActorRotation` Player)))))

(fn `Foucus/UnfocusPlayer`
  (params (YesUnFocus :type Boolean))
  (if YesUnFocus
    (`AIController.K2_SetFocus` (`AIBlueprintHelperLibrary.GetAIController` self) null)
    (set `self.PlayerIsFocused` true)
    (else
      (`AIController.K2_SetFocus` (`AIBlueprintHelperLibrary.GetAIController` self) (`self.Player`))
      (set `self.PlayerIsFocused` false))))

(fn `SetTheDamageAmount`
  (params (AttackStrength :type "/Game/Characters/MEnemy/E_AttackStrength Enum" :default "NewEnumerator0"))
  (switch `/Game/Characters/MEnemy/E_AttackStrength` AttackStrength
    (:`NewEnumerator0`
      (set `self.DamageAmount` 15.0))
    (:`NewEnumerator1`
      (set `self.DamageAmount` 30.0))
    (:`NewEnumerator2`
      (set `self.DamageAmount` 50.0))))

(fn `TeleportMaterialChange`
  (bind _mesh (`self.Mesh`))
  (`PrimitiveComponent.SetMaterial` _mesh 0 "/Game/NiagaraSystems/MM_DarkFade.MM_DarkFade")
  (`NiagaraFunctionLibrary.SpawnSystemAttached` "/Game/NiagaraSystems/NS_TeleportParticleBurst.NS_TeleportParticleBurst" _mesh "None" (0.0 0.0 0.0) (struct) "KeepRelativeOffset"))

(fn `UserConstructionScript`
  (`parent.UserConstructionScript`))