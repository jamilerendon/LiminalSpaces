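; BP_Strider is an enemy character with slam and slash-combo attacks, each exposed as a function that plays a montage.
; On BeginPlay it disables collision on its hand and knockback-scream components and hides helper meshes.
; A BehindPlayer overlap tracks the third-person player; if the flag is still set after a delay, the AI controller briefly focuses on the player, then calls SetFocus with no target.
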(event `self.ReceiveBeginPlay`
  (`parent.ReceiveBeginPlay`)
  (`PrimitiveComponent.SetCollisionEnabled` (`self.LeftHand`) "NoCollision")
  (`PrimitiveComponent.SetCollisionEnabled` (`self.KnockbackScream`) "NoCollision")
  (`PrimitiveComponent.SetCollisionEnabled` (`self.RightHand`) "NoCollision")
  (`PrimitiveComponent.SetCollisionEnabled` (`self.BothHands`) "NoCollision")
  (`SceneComponent.SetHiddenInGame` (`self.StaticMesh1`) true false)
  (`SceneComponent.SetHiddenInGame` (`self.StaticMesh`) true false)
  (`SceneComponent.SetHiddenInGame` (`self.Cube`) true false))

(event `self.BehindPlayer.OnComponentBeginOverlap`
  (params (OverlappedComponent :type "PrimitiveComponent Object Reference") (OtherActor :type "Actor Object Reference") (OtherComp :type "PrimitiveComponent Object Reference") (OtherBodyIndex :type Integer) (bFromSweep :type Boolean) (SweepResult :type "HitResult Structure (by ref)"))
  (bind _asbp_third_person_character (cast `/Game/ThirdPerson/Blueprints/BP_ThirdPersonCharacter` OtherActor))
  (set `self.Player` _asbp_third_person_character)
  (set `self.Player is Behind` true)
  (`KismetSystemLibrary.Delay` 4.0)
  (`KismetSystemLibrary.PrintString` "running event")
  (`self.SetFocusToPlayerIfPlayerIsBehindforToLong`))

(event `SetFocusToPlayerIfPlayerIsBehindforToLong`
  (if (`self.Player is Behind`)
    (`AIController.K2_SetFocus` (`AIBlueprintHelperLibrary.GetAIController` self) (`self.Player`))
    (`KismetSystemLibrary.Delay` 3.0)
    (`AIController.K2_SetFocus` (`AIBlueprintHelperLibrary.GetAIController` self) null)))

(event `self.BehindPlayer.OnComponentEndOverlap`
  (params (OverlappedComponent :type "PrimitiveComponent Object Reference") (OtherActor :type "Actor Object Reference") (OtherComp :type "PrimitiveComponent Object Reference") (OtherBodyIndex :type Integer))
  (cast `/Game/ThirdPerson/Blueprints/BP_ThirdPersonCharacter` OtherActor)
  (set `self.Player is Behind` false))

(fn `BigAttack`
  (returns (Duration :type "Float (double-precision)"))
  (bind _returnvalue (`self.PlayAnimMontage` "/Game/Characters/BossImplementation/RM_Strider/SkeletalMeshes/RM_StriderBigslam_Montage.RM_StriderBigslam_Montage"))
  (return _returnvalue))

(fn `SwordAttack`
  (returns (AnimationDuration :type "Float (double-precision)"))
  (bind _returnvalue (`self.PlayAnimMontage` "/Game/Characters/BossImplementation/RM_Strider/SkeletalMeshes/RM_StriderSlashCombo1_Montage.RM_StriderSlashCombo1_Montage"))
  (return _returnvalue))

(fn `UserConstructionScript`
  (`parent.UserConstructionScript`))