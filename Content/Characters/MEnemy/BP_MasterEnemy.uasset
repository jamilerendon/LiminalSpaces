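; Master boss enemy Blueprint that damages the third-person player and drives a named boss health bar.
; Hand and scream overlap volumes call the player's damage event; the scream uses fixed damage.
; A one-time trigger overlap has the player add the health bar, which the boss keeps and refreshes from its StatusComponent.
; When DecreaseHealth reports death, it plays a montage, fades the bar out, then removes it and destroys itself.
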(event `self.ReceiveBeginPlay`)

(event `/Game/ThirdPerson/Blueprints/I_Interactions.RecieveDamage`
  (params (DamageAmount :type "Float (double-precision)") (AttackingActor :type "Actor Object Reference"))
  (bind _as_ui_boss_health (`self.As Ui Boss Health`))
  (bind _isdead_ (`/Game/ThirdPerson/Blueprints/StatusComponent.DecreaseHealth` (`self.StatusComponent`) DamageAmount))
  (`/Game/Lwidgets/UI_BossHealthBar.RefreshHealthBar` (`self.As Ui Boss Health`) (`self.StatusComponent`))
  (if _isdead_
    (set `self.BossIsDead` true)
    (`KismetSystemLibrary.Delay` 0.2)
    (bind _returnvalue (`self.PlayAnimMontage` (`self.Who`) (`self.DeathMontage`) 1.0 "None"))
    (`UserWidget.PlayAnimationReverse` _as_ui_boss_health (`/Game/Lwidgets/UI_BossHealthBar.OpacityAnimationHealthBar` _as_ui_boss_health) 1.0 false)
    (`KismetSystemLibrary.Delay` _returnvalue)
    (`Widget.RemoveFromParent` _as_ui_boss_health)
    (`self.K2_DestroyActor`)))

(event `self.LeftHand.OnComponentBeginOverlap`
  (params (OverlappedComponent :type "PrimitiveComponent Object Reference") (OtherActor :type "Actor Object Reference") (OtherComp :type "PrimitiveComponent Object Reference") (OtherBodyIndex :type Integer) (bFromSweep :type Boolean) (SweepResult :type "HitResult Structure (by ref)"))
  (bind _asbp_third_person_character (cast `/Game/ThirdPerson/Blueprints/BP_ThirdPersonCharacter` OtherActor))
  (`/Game/ThirdPerson/Blueprints/I_Interactions.RecieveDamage` _asbp_third_person_character (`self.DamageAmount`) self))

(event `self.RightHand.OnComponentBeginOverlap`
  (params (OverlappedComponent :type "PrimitiveComponent Object Reference") (OtherActor :type "Actor Object Reference") (OtherComp :type "PrimitiveComponent Object Reference") (OtherBodyIndex :type Integer) (bFromSweep :type Boolean) (SweepResult :type "HitResult Structure (by ref)"))
  (bind _asbp_third_person_character (cast `/Game/ThirdPerson/Blueprints/BP_ThirdPersonCharacter` OtherActor))
  (`/Game/ThirdPerson/Blueprints/I_Interactions.RecieveDamage` _asbp_third_person_character (`self.DamageAmount`) self))

(event `self.BothHands.OnComponentBeginOverlap`
  (params (OverlappedComponent :type "PrimitiveComponent Object Reference") (OtherActor :type "Actor Object Reference") (OtherComp :type "PrimitiveComponent Object Reference") (OtherBodyIndex :type Integer) (bFromSweep :type Boolean) (SweepResult :type "HitResult Structure (by ref)"))
  (bind _asbp_third_person_character (cast `/Game/ThirdPerson/Blueprints/BP_ThirdPersonCharacter` OtherActor))
  (`/Game/ThirdPerson/Blueprints/I_Interactions.RecieveDamage` _asbp_third_person_character (`self.DamageAmount`) self))

(event `self.BossHealthBarAppear.OnComponentBeginOverlap`
  (params (OverlappedComponent :type "PrimitiveComponent Object Reference") (OtherActor :type "Actor Object Reference") (OtherComp :type "PrimitiveComponent Object Reference") (OtherBodyIndex :type Integer) (bFromSweep :type Boolean) (SweepResult :type "HitResult Structure (by ref)"))
  (bind _asbp_third_person_character (cast `/Game/ThirdPerson/Blueprints/BP_ThirdPersonCharacter` OtherActor))
  (`/Engine/EditorBlueprintResources/StandardMacros.DoOnce` false
    (:`Completed`
      (set `/Game/ThirdPerson/Blueprints/BP_ThirdPersonCharacter.HealthBarTitle` (`self.Boss Name`) _asbp_third_person_character)
      (`/Game/ThirdPerson/Blueprints/BP_ThirdPersonCharacter.Add Boss HealthBar to screen` _asbp_third_person_character)
      (bind _output_get (set `self.As Ui Boss Health` (`/Game/ThirdPerson/Blueprints/BP_ThirdPersonCharacter.BossHealthBar` _asbp_third_person_character)))
      (`/Game/Lwidgets/UI_BossHealthBar.RefreshHealthBar` _output_get (`self.StatusComponent`)))))

(event `self.KnockbackScream.OnComponentBeginOverlap`
  (params (OverlappedComponent :type "PrimitiveComponent Object Reference") (OtherActor :type "Actor Object Reference") (OtherComp :type "PrimitiveComponent Object Reference") (OtherBodyIndex :type Integer) (bFromSweep :type Boolean) (SweepResult :type "HitResult Structure (by ref)"))
  (bind _asbp_third_person_character (cast `/Game/ThirdPerson/Blueprints/BP_ThirdPersonCharacter` OtherActor))
  (`/Game/ThirdPerson/Blueprints/I_Interactions.RecieveDamage` _asbp_third_person_character 20.0 self))

(fn `Dying`)

(fn `UserConstructionScript`)