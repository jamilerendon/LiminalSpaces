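; Anemoia boss character, a child Blueprint with melee, lunge, scream and projectile attacks.
; Attack functions play montages and set Lunging or Throwing flags, which Tick reads through DoOnce and delays to boost walk speed or fire an eye projectile at the player.
; Helper functions toggle hand and scream hitboxes and set damage tiers.
; Several other attack functions are empty stubs, and the respawn logic in ResetBossAnemoia is disconnected.
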(event `self.ReceiveBeginPlay`
  (`parent.ReceiveBeginPlay`)
  (set `self.Boss Name` "/Game/Lwidgets/AnemoiaTitle.AnemoiaTitle")
  (`self.DisableHitboxes`)
  (`self.AttachHitboxes`)
  (set `self.Who` self)
  (set `self.DeathMontage` "/Game/Characters/BossImplementation/RM_Anemoia/SkeletalMeshes/RM_AnemoiaDeath_Montage.RM_AnemoiaDeath_Montage")
  (`SceneComponent.SetHiddenInGame` (`self.StaticMesh1`) true false)
  (`SceneComponent.SetHiddenInGame` (`self.Sphere1`) true false)
  (`SceneComponent.SetHiddenInGame` (`self.StaticMesh`) true false)
  (`SceneComponent.SetHiddenInGame` (`self.Sphere`) true false)
  (`SceneComponent.SetHiddenInGame` (`self.Cube`) true false)
  (set `self.Myself` "BP_REAnemoia_C"))

(event `self.ReceiveTick`
  (params (DeltaSeconds :type "Float (single-precision)"))
  (bind _returnvalue (`SceneComponent.GetSocketLocation` (`self.Mesh`) "EyeSocket"))
  (if (`self.Throwing`)
    (`/Engine/EditorBlueprintResources/StandardMacros.DoOnce` false :!label _label
      (:`Completed`
        (`KismetSystemLibrary.Delay` 0.5)
        (bind _returnvalue_2 (`GameplayStatics.GetActorOfClass` "/Game/ThirdPerson/Blueprints/BP_ThirdPersonCharacter.BP_ThirdPersonCharacter_C"))
        (`|SpawnActorFromClass` "/Game/Characters/BossImplementation/BP_AnemoiaProjectile.BP_AnemoiaProjectile_C" (`KismetMathLibrary.MakeTransform` (+ _returnvalue (0.0 0.0 0.0)) (`KismetMathLibrary.MakeRotFromX` (`KismetMathLibrary.Normal` (- (`SceneComponent.K2_GetComponentLocation` (`Character.Mesh` _returnvalue_2)) _returnvalue)))) "Undefined" "MultiplyWithRoot" null null)
        (`KismetSystemLibrary.Delay` 6.0)
        (`self.ResetThrow`)))
    (elif (`self.Lunging`)
      (`/Engine/EditorBlueprintResources/StandardMacros.DoOnce` false :!label _label_2
        (:`Completed`
          (`KismetSystemLibrary.Delay` 0.3)
          (set `CharacterMovementComponent.MaxWalkSpeed` 2000.0 (`self.CharacterMovement`))))
      (else
        (set `CharacterMovementComponent.MaxWalkSpeed` 400.0 (`self.CharacterMovement`))
        (`KismetSystemLibrary.Delay` 1.0)
        (`self.ResetSettingFastSpeed`)))))

(event `ResetThrow`
  (goto _label :!via `Reset`))

(event `ResetSettingFastSpeed`
  (goto _label_2 :!via `Reset`))

(event `AnemoiaResetTHeBoss`
  (`self.ResetBoss`))

(fn `ActivateBothHitbox`
  (`PrimitiveComponent.SetCollisionEnabled` (`self.BothHands`) "QueryAndProbe"))

(fn `ActivateLeftHitbox`
  (`PrimitiveComponent.SetCollisionEnabled` (`self.LeftHand`) "QueryAndProbe"))

(fn `ActivateRightHitbox`
  (`PrimitiveComponent.SetCollisionEnabled` (`self.RightHand`) "QueryAndProbe"))

(fn `ActivateScreamHitbox`
  (`PrimitiveComponent.SetCollisionEnabled` (`self.KnockbackScream`) "QueryAndPhysics"))

(fn `AHandSlam`
  (returns (Duration :type "Float (double-precision)"))
  (bind _returnvalue (`self.PlayAnimMontage` "/Game/Characters/BossImplementation/RM_Anemoia/SkeletalMeshes/RM_Anemoia1HandSlam_Montage.RM_Anemoia1HandSlam_Montage"))
  (set `self.Lunging` false)
  (set `self.Throwing` false)
  (return _returnvalue))

(fn `ALunge`
  (returns (Duration :type "Float (double-precision)"))
  (bind _returnvalue (`self.PlayAnimMontage` "/Game/Characters/BossImplementation/RM_Anemoia/SkeletalMeshes/RM_AnemoiaLunge_Montage.RM_AnemoiaLunge_Montage"))
  (set `self.Lunging` true)
  (set `self.Throwing` false)
  (return _returnvalue))

(fn `AScream`
  (returns (Duration :type "Float (double-precision)"))
  (bind _returnvalue (`self.PlayAnimMontage` "/Game/Characters/BossImplementation/RM_Anemoia/SkeletalMeshes/RM_AnemoiaScream_Montage.RM_AnemoiaScream_Montage"))
  (`NiagaraFunctionLibrary.SpawnSystemAttached` "/Game/NiagaraSystems/Shockwave/NS_Shockwave.NS_Shockwave" (`self.Mesh`) "headSocket" (0.0 0.0 0.0) (struct) "KeepRelativeOffset")
  (set `self.Throwing` false)
  (set `self.Lunging` false)
  (return _returnvalue))

(fn `ASlash1`
  (returns (Duration :type "Float (double-precision)"))
  (bind _returnvalue (`self.PlayAnimMontage` "/Game/Characters/BossImplementation/RM_Anemoia/SkeletalMeshes/RM_AnemoiaSlashCombo1_Montage.RM_AnemoiaSlashCombo1_Montage"))
  (set `self.Lunging` false)
  (set `self.Throwing` false)
  (return _returnvalue))

(fn `ASlash2`
  (returns (Duration :type "Float (double-precision)"))
  (bind _returnvalue (`self.PlayAnimMontage` "/Game/Characters/BossImplementation/RM_Anemoia/SkeletalMeshes/RM_AnemoiaSlashCombo2_Montage.RM_AnemoiaSlashCombo2_Montage"))
  (set `self.Lunging` false)
  (set `self.Throwing` false)
  (return _returnvalue))

(fn `ASlash3`
  (returns (Duration :type "Float (double-precision)"))
  (bind _returnvalue (`self.PlayAnimMontage` "/Game/Characters/BossImplementation/RM_Anemoia/SkeletalMeshes/RM_AnemoiaSlashCombo3_Montage.RM_AnemoiaSlashCombo3_Montage"))
  (set `self.Lunging` false)
  (set `self.Throwing` false)
  (return _returnvalue))

(fn `AThrow`
  (returns (Duration :type "Float (double-precision)"))
  (bind _returnvalue (`self.PlayAnimMontage` "/Game/Characters/BossImplementation/RM_Anemoia/SkeletalMeshes/RM_AnemoiaThrow_Montage.RM_AnemoiaThrow_Montage"))
  (set `self.Lunging` false)
  (set `self.Throwing` true)
  (return _returnvalue))

(fn `AttachHitboxes`
  (bind _mesh (`self.Mesh`))
  (`SceneComponent.K2_AttachToComponent` (`self.StaticMesh`) _mesh "hand_rSocket" "KeepRelative" "KeepRelative" "KeepWorld" false)
  (`SceneComponent.K2_AttachToComponent` (`self.StaticMesh1`) _mesh "rootSocket" "KeepRelative" "KeepRelative" "KeepWorld" false)
  (`SceneComponent.K2_AttachToComponent` (`self.Cube`) _mesh "hand_lSocket" "KeepRelative" "KeepRelative" "KeepWorld" false))

(fn `AUppercut`
  (returns (Duration :type "Float (double-precision)"))
  (bind _returnvalue (`self.PlayAnimMontage` "/Game/Characters/BossImplementation/RM_Anemoia/SkeletalMeshes/RM_AnemoiaUppercut_Montage.RM_AnemoiaUppercut_Montage"))
  (set `self.Lunging` false)
  (set `self.Throwing` false)
  (return _returnvalue))

(fn `BigAttack`
  (returns (Duration :type "Float (double-precision)"))
  (return 0.0))

(fn `DeactivateBothHitbox`
  (`PrimitiveComponent.SetCollisionEnabled` (`self.BothHands`) "NoCollision"))

(fn `DeactivateLeftHitbox`
  (`PrimitiveComponent.SetCollisionEnabled` (`self.LeftHand`) "NoCollision"))

(fn `DeactivateRightHitbox`
  (`PrimitiveComponent.SetCollisionEnabled` (`self.RightHand`) "NoCollision"))

(fn `DeactivateScreamHitbox`
  (`PrimitiveComponent.SetCollisionEnabled` (`self.KnockbackScream`) "NoCollision"))

(fn `DisableHitboxes`
  (`PrimitiveComponent.SetCollisionEnabled` (`self.KnockbackScream`) "NoCollision")
  (`PrimitiveComponent.SetCollisionEnabled` (`self.RightHand`) "NoCollision")
  (`PrimitiveComponent.SetCollisionEnabled` (`self.BothHands`) "NoCollision")
  (`PrimitiveComponent.SetCollisionEnabled` (`self.LeftHand`) "NoCollision"))

(fn `EyeLazer`
  (returns (Duration :type "Float (double-precision)"))
  (return 0.0))

(fn `ResetBossAnemoia`
  (if (`self.CastedToPlayer`)
    _))

(fn `Set Attack Strength Strong`
  (set `self.DamageAmount` 30.0))

(fn `Set Attack Super Strong`
  (set `self.DamageAmount` 45.0))

(fn `Set Attack Weak`
  (set `self.DamageAmount` 15.0))

(fn `SlamCombo`
  (returns (Duration :type "Float (double-precision)"))
  (return 0.0))

(fn `SlamJumpAttack`
  (returns (Duration :type "Float (double-precision)"))
  (return 0.0))

(fn `SpawnSplashEffect`
  (`NiagaraFunctionLibrary.SpawnSystemAtLocation` "/Game/NiagaraSystems/NS_Splash.NS_Splash" (`SceneComponent.GetSocketLocation` (`self.Mesh`) "rootSocket")))

(fn `SpinningAttack`
  (returns (Duration :type "Float (double-precision)"))
  (return 0.0))

(fn `SwordAttack`
  (returns (AnimationDuration :type "Float (double-precision)"))
  (return 0.0))

(fn `UserConstructionScript`
  (`parent.UserConstructionScript`))