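; NPC Blueprint that runs a voiced dialogue when the third-person character enters its sphere.
; Overlap registers the NPC on the player and shows the dialogue widget, while leaving or running out of lines hides it and resets.
; NextLine steps through DT_NPCDialogue rows in order, playing audio and tilting and justifying text by speaker.
; An older array-based version remains unconnected.
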(event `self.ReceiveBeginPlay`
  (bind _returnvalue (`|CreateWidget` "/Game/Widgets/W_NPCDialogue.W_NPCDialogue_C")) ; Get the widget ready to show
  (set `self.W_Dialogue` _returnvalue)
  (set `self.NextLineIndex` (`self.IndexStart`)))

(event `self.Sphere.OnComponentBeginOverlap`
  (params (OverlappedComponent :type "PrimitiveComponent Object Reference") (OtherActor :type "Actor Object Reference") (OtherComp :type "PrimitiveComponent Object Reference") (OtherBodyIndex :type Integer) (bFromSweep :type Boolean) (SweepResult :type "HitResult Structure (by ref)"))
  (bind _asbp_third_person_character (cast `/Game/ThirdPerson/Blueprints/BP_ThirdPersonCharacter` OtherActor))
  (bind _output_get (set `self.Player` _asbp_third_person_character))
  (set `/Game/ThirdPerson/Blueprints/BP_ThirdPersonCharacter.NPC` self _output_get) ; Tell the plater that they're talking to us
  (`UserWidget.AddToViewport` (`self.W_Dialogue`) 0)
  (`self.Next Line`))

(event `self.Sphere.OnComponentEndOverlap`
  (params (OverlappedComponent :type "PrimitiveComponent Object Reference") (OtherActor :type "Actor Object Reference") (OtherComp :type "PrimitiveComponent Object Reference") (OtherBodyIndex :type Integer))
  (cast `/Game/ThirdPerson/Blueprints/BP_ThirdPersonCharacter` OtherActor)
  (`self.End Dialogue`))

(event `End Dialogue`
  (`Widget.RemoveFromParent` (`self.W_Dialogue`)) ; Hide the dialogue
  (set `self.NextLineIndex` (`self.IndexStart`)) ; Reset the Index
  (set `/Game/ThirdPerson/Blueprints/BP_ThirdPersonCharacter.NPC` null (`self.Player`)) ; Set NPC to nothing, tell the player to forget about us.
  (set `self.Player` null) ; Set Player to nothing
)

(event `Next Line`
  (bind _audiocomponent (`self.AudioComponent`))
  (bind _textblock_0 (`/Game/Widgets/W_NPCDialogue.TextBlock_0` (`self.W_Dialogue`)))
  (bind _outrownames (`DataTableFunctionLibrary.GetDataTableRowNames` "/Game/Blueprints/DT_NPCDialogue.DT_NPCDialogue"))
  (if (> (`self.NextLineIndex`) (`KismetArrayLibrary.Array_LastIndex` _outrownames))
    (`self.End Dialogue`)
    (else
      (bind _returnvalue (`|GetDataTableRow` "/Game/Blueprints/DT_NPCDialogue.DT_NPCDialogue" (`|GetArrayItem` _outrownames (`self.NextLineIndex`)))
        (:`then`
          (`TextBlock.SetText` (`/Game/Widgets/W_NPCDialogue.TextBlock_0` (`self.W_Dialogue`)) (`KismetTextLibrary.Conv_StringToText` (break `/Game/Blueprints/S_NPCDialogue` _returnvalue))) ; Shows the next line
          (`/Engine/EditorBlueprintResources/StandardMacros.IncrementInt` (`self.NextLineIndex`) ; Increment Int
            (:`  `
              ; Play Audio, canceling previous lines if needed
              (`AudioComponent.SetSound` _audiocomponent (`.VoicedLine_9_7DBFA60444324F24E24EB49827D27E2D` (break `/Game/Blueprints/S_NPCDialogue` _returnvalue)))
              (`AudioComponent.Play` _audiocomponent 0.0)
              (switch `/Game/Blueprints/E_Speaker` (`.Speaker_10_90C924CA4074D3B0E40A3EBFEBDCE567` (break `/Game/Blueprints/S_NPCDialogue` _returnvalue))
                (:`NewEnumerator0`
                  (`Widget.SetRenderTransformAngle` _textblock_0 (`KismetMathLibrary.RandomFloatInRange` -5.5 -4.5))
                  (set `TextLayoutWidget.Justification` "Left" _textblock_0) ; Set Justification
                )
                (:`NewEnumerator1`
                  (`Widget.SetRenderTransformAngle` _textblock_0 (`KismetMathLibrary.RandomFloatInRange` 4.5 5.5))
                  (set `TextLayoutWidget.Justification` "Right" _textblock_0) ; Set Justification
                )))))))))

(fn `UserConstructionScript`)