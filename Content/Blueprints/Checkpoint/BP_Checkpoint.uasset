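; BP_Checkpoint is a checkpoint actor that saves the player's progress when the third-person character enters its collision.
; On overlap it stores its root transform as the character's LastCheckpoint, calls the character's Save, and swaps a material on its monitor mesh.
; The construction script assigns a texture render target to its SceneCaptureComponent2D.
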(event `self.Col_Checkpoint.OnComponentBeginOverlap`
  (params (OverlappedComponent :type "PrimitiveComponent Object Reference") (OtherActor :type "Actor Object Reference") (OtherComp :type "PrimitiveComponent Object Reference") (OtherBodyIndex :type Integer) (bFromSweep :type Boolean) (SweepResult :type "HitResult Structure (by ref)"))
  (bind _asbp_third_person_character (cast `/Game/ThirdPerson/Blueprints/BP_ThirdPersonCharacter` OtherActor))
  (bind _output_get (set `self.Player` _asbp_third_person_character))
  (set `/Game/ThirdPerson/Blueprints/BP_ThirdPersonCharacter.LastCheckpoint` (`SceneComponent.K2_GetComponentToWorld` (`self.DefaultSceneRoot`)) _output_get)
  (`/Game/ThirdPerson/Blueprints/BP_ThirdPersonCharacter.Save` _asbp_third_person_character)
  (`PrimitiveComponent.SetMaterial` (`self.SM_Monitor`) 1 (`self.Material`)))

(fn `UserConstructionScript`
  (set `SceneCaptureComponent2D.TextureTarget` (`self.Texture Target`) (`self.SceneCaptureComponent2D`)))