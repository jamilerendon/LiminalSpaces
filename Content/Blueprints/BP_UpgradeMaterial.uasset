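; BP_UpgradeMaterial is a pickup that adds one upgrade material to the BP_ThirdPersonCharacter that collects it.
; Tick spins the Plane on pitch by incrementing Rotation each frame, independent of delta time.
; Sphere overlap runs through a DoOnce ahead of the character cast, increments UpgradeMats, then after short delays activates Niagara, shows an animated WBP_WeaponShard widget and destroys the actor.
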(event `self.ReceiveTick`
  (params (DeltaSeconds :type "Float (single-precision)"))
  (bind _result (`/Engine/EditorBlueprintResources/StandardMacros.IncrementFloat` (`self.Rotation`))
    (:`  `
      (bind _output_get (set `self.Rotation` _result))
      (`SceneComponent.K2_SetRelativeRotation` (`self.Plane`) (`KismetMathLibrary.MakeRotator` 0.0 _output_get) false false))))

(event `self.Sphere.OnComponentBeginOverlap`
  (params (OverlappedComponent :type "PrimitiveComponent Object Reference") (OtherActor :type "Actor Object Reference") (OtherComp :type "PrimitiveComponent Object Reference") (OtherBodyIndex :type Integer) (bFromSweep :type Boolean) (SweepResult :type "HitResult Structure (by ref)"))
  (`/Engine/EditorBlueprintResources/StandardMacros.DoOnce` false
    (:`Completed`
      (bind _asbp_third_person_character (cast `/Game/ThirdPerson/Blueprints/BP_ThirdPersonCharacter` OtherActor))
      (set `/Game/ThirdPerson/Blueprints/BP_ThirdPersonCharacter.UpgradeMats` (+ (`/Game/ThirdPerson/Blueprints/BP_ThirdPersonCharacter.UpgradeMats` _asbp_third_person_character) 1.0) _asbp_third_person_character)
      (`KismetSystemLibrary.Delay` 0.2)
      (`ActorComponent.Activate` (`self.Niagara`) false)
      (bind _returnvalue (`|CreateWidget` "/Game/Lwidgets/WBP_WeaponShard.WBP_WeaponShard_C"))
      (bind _output_get (set `self.WeaponSHard` _returnvalue))
      (`UserWidget.AddToViewport` _output_get 0)
      (`UserWidget.PlayAnimation` _output_get (`/Game/Lwidgets/WBP_WeaponShard.OpacityAnimation` _output_get) 0.0 1 "Forward" 1.0 false)
      (`KismetSystemLibrary.Delay` 2.0)
      (`self.K2_DestroyActor`))))

(fn `UserConstructionScript`)