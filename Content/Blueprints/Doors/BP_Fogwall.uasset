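; BP_Fogwall is a fog wall barrier that the player can dismiss and that returns while a boss health bar is active.
; Box overlap caches the third-person character and toggles its fogwall widget.
; KillWidget, effective only during overlap, hides the wall, disables Box and Cube collision and removes the widget.
; Once it has met the player, Tick polls the character's boss health bar flags and restores visibility and collision.
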(event `Reemmerge`
  (`self.SetActorHiddenInGame` false)
  (`PrimitiveComponent.SetCollisionEnabled` (`self.Box`) "QueryAndPhysics")
  (`PrimitiveComponent.SetCollisionEnabled` (`self.Cube`) "QueryAndPhysics")
  (set `self.FogwallIsDisable` false))

(event `self.ReceiveTick`
  (params (DeltaSeconds :type "Float (single-precision)"))
  (bind _as_bp_third_person_character (`self.As BP Third Person Character`))
  (if (`self.HasMetPlayer`)
    (if (and (`/Game/ThirdPerson/Blueprints/BP_ThirdPersonCharacter.AddedBossHealthBar` _as_bp_third_person_character) (not (`/Game/ThirdPerson/Blueprints/BP_ThirdPersonCharacter.RemovedBossHealthBar` _as_bp_third_person_character)))
      (`self.Reemmerge`))))

(event `self.Box.OnComponentBeginOverlap`
  (params (OverlappedComponent :type "PrimitiveComponent Object Reference") (OtherActor :type "Actor Object Reference") (OtherComp :type "PrimitiveComponent Object Reference") (OtherBodyIndex :type Integer) (bFromSweep :type Boolean) (SweepResult :type "HitResult Structure (by ref)"))
  (bind _asbp_third_person_character (cast `/Game/ThirdPerson/Blueprints/BP_ThirdPersonCharacter` OtherActor))
  (bind _output_get (set `self.As BP Third Person Character` _asbp_third_person_character))
  (`/Game/ThirdPerson/Blueprints/BP_ThirdPersonCharacter.AddFogwallWidgetToViewport` _output_get)
  (set `self.is overlapping` true)
  (set `self.HasMetPlayer` true))

(event `self.Box.OnComponentEndOverlap`
  (params (OverlappedComponent :type "PrimitiveComponent Object Reference") (OtherActor :type "Actor Object Reference") (OtherComp :type "PrimitiveComponent Object Reference") (OtherBodyIndex :type Integer))
  (bind _asbp_third_person_character (cast `/Game/ThirdPerson/Blueprints/BP_ThirdPersonCharacter` OtherActor))
  (`/Game/ThirdPerson/Blueprints/BP_ThirdPersonCharacter.RemoveFogwallWidgetFromViewport` _asbp_third_person_character)
  (set `self.is overlapping` false))

(event `KillWidget`
  (if (and (`self.HasMetPlayer`) (`self.is overlapping`))
    (`self.SetActorHiddenInGame` true)
    (`PrimitiveComponent.SetCollisionEnabled` (`self.Box`) "NoCollision")
    (`PrimitiveComponent.SetCollisionEnabled` (`self.Cube`) "NoCollision")
    (`/Game/ThirdPerson/Blueprints/BP_ThirdPersonCharacter.RemoveFogwallWidgetFromViewport` (`self.As BP Third Person Character`))
    (set `self.FogwallIsDisable` true)))

(fn `UserConstructionScript`)