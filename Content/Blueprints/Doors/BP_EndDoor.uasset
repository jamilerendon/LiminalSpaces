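; BP_EndDoor is the exit door that appears after the boss dies and quits the game when the player enters it.
; It starts hidden with trigger collision off, then polls BP_Strider's BossIsDead flag on Tick and reveals itself once through a DoOnce.
; When BP_ThirdPersonCharacter overlaps the trigger, it shows the WB_FadingDoor fade widget, plays a door sound and quits after a short delay.
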(event `self.ReceiveBeginPlay`
  (bind _returnvalue (`GameplayStatics.GetActorOfClass` "/Game/Characters/MEnemy/BP_Strider.BP_Strider_C"))
  (set `self.The Strider` _returnvalue)
  (`self.SetActorHiddenInGame` true)
  (`PrimitiveComponent.SetCollisionEnabled` (`self.Trigger`) "NoCollision"))

(event `self.ReceiveTick`
  (params (DeltaSeconds :type "Float (single-precision)"))
  (if (`/Game/Characters/MEnemy/BP_MasterEnemy.BossIsDead` (`self.The Strider`))
    (`/Engine/EditorBlueprintResources/StandardMacros.DoOnce` false
      (:`Completed`
        (`self.SetActorHiddenInGame` false)
        (`PrimitiveComponent.SetCollisionEnabled` (`self.Trigger`) "QueryAndPhysics")))))

(event `self.Trigger.OnComponentBeginOverlap`
  (params (OverlappedComponent :type "PrimitiveComponent Object Reference") (OtherActor :type "Actor Object Reference") (OtherComp :type "PrimitiveComponent Object Reference") (OtherBodyIndex :type Integer) (bFromSweep :type Boolean) (SweepResult :type "HitResult Structure (by ref)"))
  (cast `/Game/ThirdPerson/Blueprints/BP_ThirdPersonCharacter` OtherActor)
  (bind _returnvalue (`|CreateWidget` "/Game/Widgets/WB_FadingDoor.WB_FadingDoor_C"))
  (`UserWidget.AddToViewport` _returnvalue 0)
  (`/Game/Widgets/WB_FadingDoor.Fade Anim` _returnvalue)
  (`GameplayStatics.PlaySound2D` "/Game/Audio/SoundWaves/SC_DoorOpen_Cue.SC_DoorOpen_Cue" 1.0 1.0 0.0 null null)
  (`KismetSystemLibrary.Delay` 0.5)
  (`KismetSystemLibrary.QuitGame` null "Quit"))

(fn `UserConstructionScript`)