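; Anvil actor that upgrades the player's weapon when the third-person character overlaps its Upgrade component while holding upgrade materials.
; The hammer mesh starts hidden, then appears and plays its strike animation three times at three-second intervals, activating a Niagara effect with each play.
; The character's UpgradeWeapon runs as the animation starts, behind a DoOnce that resets 0.2 seconds later.
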(event `self.ReceiveBeginPlay`
  (`SceneComponent.SetHiddenInGame` (`self.AnimatedLinimalHammer`) true false))

(event `Play Hammer animation`
  (`SceneComponent.SetHiddenInGame` (`self.AnimatedLinimalHammer`) false false)
  (`SkeletalMeshComponent.PlayAnimation` (`self.AnimatedLinimalHammer`) "/Game/Imported/AnimatedLinimalHammer/SkeletalMeshes/AnimatedLinimalHammer_Anim.AnimatedLinimalHammer_Anim" false)
  (`ActorComponent.Activate` (`self.Niagara`) false)
  (`KismetSystemLibrary.Delay` 3.0)
  (`SkeletalMeshComponent.PlayAnimation` (`self.AnimatedLinimalHammer`) "/Game/Imported/AnimatedLinimalHammer/SkeletalMeshes/AnimatedLinimalHammer_Anim.AnimatedLinimalHammer_Anim" false)
  (`ActorComponent.Activate` (`self.Niagara`) false)
  (`KismetSystemLibrary.Delay` 3.0)
  (`SkeletalMeshComponent.PlayAnimation` (`self.AnimatedLinimalHammer`) "/Game/Imported/AnimatedLinimalHammer/SkeletalMeshes/AnimatedLinimalHammer_Anim.AnimatedLinimalHammer_Anim" false)
  (`ActorComponent.Activate` (`self.Niagara`) false))

(event `self.Upgrade.OnComponentBeginOverlap`
  (params (OverlappedComponent :type "PrimitiveComponent Object Reference") (OtherActor :type "Actor Object Reference") (OtherComp :type "PrimitiveComponent Object Reference") (OtherBodyIndex :type Integer) (bFromSweep :type Boolean) (SweepResult :type "HitResult Structure (by ref)"))
  (bind _asbp_third_person_character (cast `/Game/ThirdPerson/Blueprints/BP_ThirdPersonCharacter` OtherActor))
  (if (> (`/Game/ThirdPerson/Blueprints/BP_ThirdPersonCharacter.UpgradeMats` _asbp_third_person_character) 0.0)
    (`/Engine/EditorBlueprintResources/StandardMacros.DoOnce` false :!label _label
      (:`Completed`
        (`self.Play Hammer animation`)
        (`/Game/ThirdPerson/Blueprints/BP_ThirdPersonCharacter.UpgradeWeapon` _asbp_third_person_character)
        (`KismetSystemLibrary.Delay` 0.2)
        (`self.Done Upgrading`)))))

(event `Done Upgrading`
  (goto _label :!via `Reset`))

(fn `UserConstructionScript`)