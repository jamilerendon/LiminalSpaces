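; NPC Blueprint that runs voiced, subtitled dialogue with the player while they are inside its sphere.
; Overlap shows a portrait widget created at BeginPlay and registers the NPC on the third-person character.
; NextLine steps through DT_NPC_Dialogue rows from a starting index, playing audio and setting text alignment and animation by speaker.
; An end-of-line marker, or running out of rows, closes the widget and resets the index.
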(event `self.ReceiveBeginPlay`
  (bind _npcdialogewidget (`self.NPCDialogeWidget`))
  (bind _returnvalue (`|CreateWidget` "/Game/NPCWidgets/W_NPC_Dialoge.W_NPC_Dialoge_C")) ; Get The widget ready to show
  (set `self.NPCDialogeWidget` _returnvalue)
  (set `self.NextLineIndex` (`self.StartingLineIndex`))
  (bind _npcportrait (`self.NPCPortrait`)
    (:`then`
      (`Image.SetBrushFromTexture` (`/Game/NPCWidgets/W_NPC_Dialoge.Image` _npcdialogewidget) _npcportrait false)
      (bind _playerportrait (`self.Playerportrait`)
        (:`then`
          (`Image.SetBrushFromTexture` (`/Game/NPCWidgets/W_NPC_Dialoge.Image_0` _npcdialogewidget) _playerportrait false))
        (:`else`)))
    (:`else`)))

(event `Remove Widget from Viewport`
  (`Widget.RemoveFromParent` (`self.NPCDialogeWidget`)))

(event `self.Sphere.OnComponentBeginOverlap`
  (params (OverlappedComponent :type "PrimitiveComponent Object Reference") (OtherActor :type "Actor Object Reference") (OtherComp :type "PrimitiveComponent Object Reference") (OtherBodyIndex :type Integer) (bFromSweep :type Boolean) (SweepResult :type "HitResult Structure (by ref)"))
  (bind _asbp_third_person_character (cast `/Game/ThirdPerson/Blueprints/BP_ThirdPersonCharacter` OtherActor))
  (bind _output_get (set `self.Player` _asbp_third_person_character))
  (`UserWidget.AddToViewport` (`self.NPCDialogeWidget`) 0)
  (set `/Game/ThirdPerson/Blueprints/BP_ThirdPersonCharacter.NPC` self _output_get))

(event `self.Sphere.OnComponentEndOverlap`
  (params (OverlappedComponent :type "PrimitiveComponent Object Reference") (OtherActor :type "Actor Object Reference") (OtherComp :type "PrimitiveComponent Object Reference") (OtherBodyIndex :type Integer))
  (bind _asbp_third_person_character (cast `/Game/ThirdPerson/Blueprints/BP_ThirdPersonCharacter` OtherActor))
  (set `/Game/ThirdPerson/Blueprints/BP_ThirdPersonCharacter.NPC` null _asbp_third_person_character)
  (set `self.Player` null)
  (`self.Remove Widget from Viewport`))

(event `End Dialouge`
  (set `/Game/ThirdPerson/Blueprints/BP_ThirdPersonCharacter.NPC` null (`self.Player`))
  (set `self.Player` null)
  (`self.Remove Widget from Viewport`)
  (set `self.NextLineIndex` (`self.StartingLineIndex`)))

(event `Next Line`
  (bind _npcdialogewidget (`self.NPCDialogeWidget`))
  (bind _audio (`self.Audio`))
  (bind _textblock_0 (`/Game/NPCWidgets/W_NPC_Dialoge.TextBlock_0` _npcdialogewidget))
  (bind _outrownames (`DataTableFunctionLibrary.GetDataTableRowNames` "/Game/NPCSetup/DT_NPC_Dialogue.DT_NPC_Dialogue"))
  (if (> (`self.NextLineIndex`) (`KismetArrayLibrary.Array_LastIndex` _outrownames))
    (`self.End Dialouge`)
    (else
      (bind _returnvalue (`|GetDataTableRow` "/Game/NPCSetup/DT_NPC_Dialogue.DT_NPC_Dialogue" (`|GetArrayItem` _outrownames (`self.NextLineIndex`)))
        (:`then`
          (if (`KismetStringLibrary.EqualEqual_StrStr` (break `/Game/NPCSetup/S_NPCDialogue` _returnvalue) "<end-of-line>")
            (`self.End Dialouge`)
            (else
              (`AudioComponent.SetSound` _audio (`.VoicedLine_7_01B6D1894D7D8BEC8A2E54838E3E6640` (break `/Game/NPCSetup/S_NPCDialogue` _returnvalue)))
              (`AudioComponent.Play` _audio 0.0)
              (`TextBlock.SetText` (`/Game/NPCWidgets/W_NPC_Dialoge.TextBlock_0` _npcdialogewidget) (`KismetTextLibrary.Conv_StringToText` (break `/Game/NPCSetup/S_NPCDialogue` _returnvalue)))
              (if (`|EnumEquality` (`.Speaker_8_9F83EC70483FC1DF40462DA10DA92682` (break `/Game/NPCSetup/S_NPCDialogue` _returnvalue)) "NewEnumerator0")
                (set `TextLayoutWidget.Justification` "Right" _textblock_0)
                (bind _result (`/Engine/EditorBlueprintResources/StandardMacros.IncrementInt` (`self.NextLineIndex`))
                  (:`  `
                    (set `self.NextLineIndex` _result)
                    (`UserWidget.PlayAnimation` _npcdialogewidget (`/Game/NPCWidgets/W_NPC_Dialoge.ImageAnim2` _npcdialogewidget) 0.0 1 "Forward" 1.0 false)))
                (else
                  (set `TextLayoutWidget.Justification` "Left" _textblock_0)
                  (bind _result_2 (`/Engine/EditorBlueprintResources/StandardMacros.IncrementInt` (`self.NextLineIndex`))
                    (:`  `
                      (set `self.NextLineIndex` _result_2)
                      (`UserWidget.PlayAnimation` _npcdialogewidget (`/Game/NPCWidgets/W_NPC_Dialoge.ImageAnim` _npcdialogewidget) 0.0 1 "Forward" 1.0 false))))))))))))

(fn `UserConstructionScript`)